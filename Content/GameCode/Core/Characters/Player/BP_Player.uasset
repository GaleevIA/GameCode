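; BP_Player is the player character Blueprint, adding a camera distance change while sprinting.
; It caches the spring arm's default length on BeginPlay and extends the parent's sprint start and end events.
; A timeline plays on sprint start and reverses on sprint end, lerping the arm length between the default and sprint values for a smooth transition.
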(event EventBeginPlay
  (Variables|Default|SetDefaultArmLength (Variables|/Script/Engine.SpringArmComponent|GetTargetArmLength (Variables|Default|GetSpringArmComponent))))

(event EventOnSprintStart
  (|CallParentFunction)
  (bind _newtrack_0 (Timeline|Timeline_0 Play)
    (:Update
      (Variables|/Script/Engine.SpringArmComponent|SetTargetArmLength (Variables|Default|GetSpringArmComponent) (Math|Float|Lerp (Variables|Default|GetDefaultArmLength) (Variables|Default|GetSprintArmLength) _newtrack_0)))))

(event EventOnSprintEnd
  (|CallParentFunction)
  (bind _newtrack_0 (Timeline|Timeline_0 Reverse)
    (:Update
      (Variables|/Script/Engine.SpringArmComponent|SetTargetArmLength (Variables|Default|GetSpringArmComponent) (Math|Float|Lerp (Variables|Default|GetDefaultArmLength) (Variables|Default|GetSprintArmLength) _newtrack_0)))))

(fn ConstructionScript)